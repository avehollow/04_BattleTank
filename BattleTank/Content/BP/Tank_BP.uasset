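; Player-controlled tank Blueprint that wires input and components for aiming, firing and driving.
; On BeginPlay it hands the barrel and turret to the TankAiming component and the left and right tracks to TankMovement.
; Aim axes rotate the azimuth gimbal and spring arm to steer the camera, without frame-time scaling.
; Fire calls TankAiming, while move and turn axes pass intent to TankMovement.
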(event `self.ReceiveBeginPlay`
  (`TankAimingComponent.Initialize` (`self.TankAiming`) (`self.TankBarrel`) (`self.TankTurret`))
  (`TankMovement.Initialize` (`self.TankMovement`) (`self.LeftTankTrack`) (`self.RightTankTrack`)))

(event `InputAxis|AimAzimuth`
  (params (AxisValue :type "Float (single-precision)"))
  ;[1 1 1] Dont need multiply via FrameTime because Axis Value already have value multiply by frametime
  (`SceneComponent.K2_AddLocalRotation` (`self.Azimuth Gimbal`) (`KismetMathLibrary.MakeRotator` 0.0 0.0 AxisValue) false false))

(event `InputAxis|AimElevation`
  (params (AxisValue :type "Float (single-precision)"))
  (`SceneComponent.K2_AddLocalRotation` (`self.SpringArm`) (`KismetMathLibrary.MakeRotator` 0.0 AxisValue) false false))

(event `InputAction|Fire/LMB`
  (params (Key :type "Key Structure"))
  (:`Pressed`
    (`TankAimingComponent.Fire` (`self.TankAiming`))))

(event `InputAxis|MoveFoward`
  (params (AxisValue :type "Float (single-precision)"))
  (`TankMovement.IntendMoveFoward` (`self.TankMovement`) AxisValue))

(event `InputAxis|TurnRight`
  (params (AxisValue :type "Float (single-precision)"))
  (`TankMovement.IntendTurnRight` (`self.TankMovement`) AxisValue))

(fn `UserConstructionScript`)